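; Enemy actor that hurts whatever its Cube hits and awards the player a point when it takes damage.
; A Cube hit applies damage to the other actor, then destroys the enemy.
; Any damage received increments Points on BP_Player, sets its point-increase tint flag and destroys the enemy, with no health tracking.
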(event OnComponentHit(Cube)
  (params (HitComponent :type Primitive%20Component%20Object%20Reference) (OtherActor :type Actor%20Object%20Reference) (OtherComp :type Primitive%20Component%20Object%20Reference) (NormalImpulse :type Vector :default "0, 0, 0") (Hit :type Hit%20Result%20Structure%20%28by%20ref%29))
  (Utilities|FlowControl|Sequence
    (:then_0
      (Game|Damage|ApplyDamage OtherActor 1.0 0 0))
    (:then_1
      (Actor|DestroyActor))))

(event EventBeginPlay)

(event Collision|EventActorBeginOverlap
  (params (OtherActor :type Actor%20Object%20Reference)))

(event EventTick
  (params (DeltaSeconds :type Float%20%28single-precision%29)))

(event Game|Damage|EventAnyDamage
  (params (Damage :type Float%20%28single-precision%29) (DamageType :type Damage%20Type%20Object%20Reference) (InstigatedBy :type Controller%20Object%20Reference) (DamageCauser :type Actor%20Object%20Reference))
  (Utilities|FlowControl|Sequence
    (:then_0
      (bind _asbp_player (Utilities|Casting|CastToBP_Player (Game|Player|GetPlayerPawn 0)))
      (Variables|/Game/InfiniteMatrix/Blueprints/BP_Player.BP_Player_C|SetPoints _asbp_player (+ (Variables|/Game/InfiniteMatrix/Blueprints/BP_Player.BP_Player_C|GetPoints _asbp_player) 1))
      (Variables|/Game/InfiniteMatrix/Blueprints/BP_Player.BP_Player_C|SetShowPointIncreaseTint _asbp_player true))
    (:then_1
      (Actor|DestroyActor))))

(fn ConstructionScript)