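; Bullet is a projectile actor that deals damage to whatever it hits.
; Every Tick it adds the player pawn's ForwardSpeed to the ProjectileMovement initial and max speeds, so both values accumulate over the bullet's lifetime rather than being offset once at spawn.
; When its Sphere component registers a hit, it applies a fixed damage to the other actor and destroys itself.
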(event OnComponentHit(Sphere)
  (params (HitComponent :type Primitive%20Component%20Object%20Reference) (OtherActor :type Actor%20Object%20Reference) (OtherComp :type Primitive%20Component%20Object%20Reference) (NormalImpulse :type Vector :default "0, 0, 0") (Hit :type Hit%20Result%20Structure%20%28by%20ref%29))
  (Utilities|FlowControl|Sequence
    (:then_0
      (Game|Damage|ApplyDamage OtherActor 1.0 0 0))
    (:then_1
      (Actor|DestroyActor))))

(event EventBeginPlay)

(event Collision|EventActorBeginOverlap
  (params (OtherActor :type Actor%20Object%20Reference)))

(event EventTick
  (params (DeltaSeconds :type Float%20%28single-precision%29))
  (bind _projectilemovement (Variables|Default|GetProjectileMovement))
  (bind _asbp_player (Utilities|Casting|CastToBP_Player (Game|Player|GetPlayerPawn 0)))
  (Utilities|FlowControl|Sequence
    (:then_0
      (Variables|/Script/Engine.ProjectileMovementComponent|SetInitialSpeed _projectilemovement (+ (Variables|/Script/Engine.ProjectileMovementComponent|GetInitialSpeed _projectilemovement) (Variables|/Game/InfiniteMatrix/Blueprints/BP_Player.BP_Player_C|GetForwardSpeed%20 _asbp_player))))
    (:then_1
      (Variables|/Script/Engine.ProjectileMovementComponent|SetMaxSpeed _projectilemovement (+ (Class|MovementComponent|GetMaxSpeed _projectilemovement) (Variables|/Game/InfiniteMatrix/Blueprints/BP_Player.BP_Player_C|GetForwardSpeed%20 _asbp_player))))))

(fn ConstructionScript)